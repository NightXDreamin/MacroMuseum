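; Weapon component that equips and unequips rifles and pistols on the player character, cached from player index 0 at BeginPlay.
; Rifle and Pistol events store the weapon class and overlay state, then branch on an Equip or Unequip state.
; Each branch sets that weapon's Child Actor class and snaps it to HeldObjectRoot when equipped or its Rifle/Pistol component when unequipped, then updates the character's overlay state.
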(event `self.ReceiveBeginPlay`
  (bind _asplayer (cast `/Game/TPS/TPS_Main/Player/Player` (`GameplayStatics.GetPlayerCharacter` 0)))
  (set `self.Character` _asplayer))

(event `Rifle`
  (params (WeaponBase :type "/Game/TPS/TPS_Main/Weapon/BP_WeaponBase Class Reference") (OverlayState :type "/Game/TPS/AdvancedLocomotionV4/Data/Enums/ALS_OverlayState Enum" :default "NewEnumerator0") (State :type "/Game/TPS/TPS_Main/Weapon/EWeaponState Enum" :default "NewEnumerator0"))
  (set `self.Weapon Base` WeaponBase)
  (set `self.Overlay State` OverlayState)
  (switch `/Game/TPS/TPS_Main/Weapon/EWeaponState` State
    (:`NewEnumerator0`
      (`self.RifleEquip`))
    (:`NewEnumerator1`
      (`self.RifleUnequip`))))

(event `Pistol`
  (params (WeaponBase :type "/Game/TPS/TPS_Main/Weapon/BP_WeaponBase Class Reference") (OverlayState :type "/Game/TPS/AdvancedLocomotionV4/Data/Enums/ALS_OverlayState Enum" :default "NewEnumerator0") (State :type "/Game/TPS/TPS_Main/Weapon/EWeaponState Enum" :default "NewEnumerator0"))
  (set `self.Weapon Base` WeaponBase)
  (set `self.Overlay State` OverlayState)
  (switch `/Game/TPS/TPS_Main/Weapon/EWeaponState` State
    (:`NewEnumerator0`
      (`self.PistolEquip`))
    (:`NewEnumerator1`
      (`self.PistolUnequip`))))

(fn `PistolEquip`
  (bind _character (`self.Character`))
  (bind _pistolchild (`/Game/TPS/TPS_Main/Player/Player.PistolChild` _character))
  (`ChildActorComponent.SetChildActorClass` _pistolchild (`self.Weapon Base`))
  (`SceneComponent.K2_AttachToComponent` _pistolchild (`/Game/TPS/TPS_Main/Player/Player.HeldObjectRoot` _character) "None" "SnapToTarget" "SnapToTarget" "SnapToTarget" true)
  (`/Game/TPS/TPS_Main/Player/Base_Player.BPI_Set_OverlayState` (`self.Character`) (`self.Overlay State`)))

(fn `PistolUnequip`
  (bind _character (`self.Character`))
  (bind _pistolchild (`/Game/TPS/TPS_Main/Player/Player.PistolChild` _character))
  (`ChildActorComponent.SetChildActorClass` _pistolchild (`self.Weapon Base`))
  (`SceneComponent.K2_AttachToComponent` _pistolchild (`/Game/TPS/TPS_Main/Player/Player.Pistol` _character) "None" "SnapToTarget" "SnapToTarget" "SnapToTarget" true)
  (`/Game/TPS/TPS_Main/Player/Base_Player.BPI_Set_OverlayState` (`self.Character`) (`self.Overlay State`)))

(fn `RifleEquip`
  (bind _character (`self.Character`))
  (bind _riflechild (`/Game/TPS/TPS_Main/Player/Player.RifleChild` _character))
  (`ChildActorComponent.SetChildActorClass` _riflechild (`self.Weapon Base`))
  (`SceneComponent.K2_AttachToComponent` _riflechild (`/Game/TPS/TPS_Main/Player/Player.HeldObjectRoot` _character) "None" "SnapToTarget" "SnapToTarget" "SnapToTarget" true)
  (`/Game/TPS/TPS_Main/Player/Base_Player.BPI_Set_OverlayState` (`self.Character`) (`self.Overlay State`)))

(fn `RifleUnequip`
  (bind _character (`self.Character`))
  (bind _riflechild (`/Game/TPS/TPS_Main/Player/Player.RifleChild` _character))
  (`ChildActorComponent.SetChildActorClass` _riflechild (`self.Weapon Base`))
  (`SceneComponent.K2_AttachToComponent` _riflechild (`/Game/TPS/TPS_Main/Player/Player.Rifle` _character) "None" "SnapToTarget" "SnapToTarget" "SnapToTarget" true)
  (`/Game/TPS/TPS_Main/Player/Base_Player.BPI_Set_OverlayState` (`self.Character`) (`self.Overlay State`)))