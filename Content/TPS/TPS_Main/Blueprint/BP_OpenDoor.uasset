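; BP_OpenDoor is an interactable door that shows an on-screen widget while the player is near it.
; TriggerBox overlaps with player character 0 create WBP_OpenDoor and add it to the viewport, then remove it on exit.
; The Interact event alternates a FlipFlop and passes its state to ToggleDoor, whose implementation is not in these graphs.
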(event `/Game/TPS/TPS_Main/Blueprint/BPI/BPI_Interact.Interact`
  (bind _isa (`/Engine/EditorBlueprintResources/StandardMacros.FlipFlop`)
    (:`A`
      _)
    (:`B`
      _))
  (`self.ToggleDoor` _isa))

(event `self.TriggerBox.OnComponentBeginOverlap`
  (params (OverlappedComponent :type "PrimitiveComponent Object Reference") (OtherActor :type "Actor Object Reference") (OtherComp :type "PrimitiveComponent Object Reference") (OtherBodyIndex :type Integer) (bFromSweep :type Boolean) (SweepResult :type "HitResult Structure (by ref)"))
  (if (== OtherActor (`GameplayStatics.GetPlayerCharacter` 0))
    (bind _returnvalue (`|CreateWidget` "/Game/TPS/TPS_Main/UI/WBP_OpenDoor.WBP_OpenDoor_C"))
    (`UserWidget.AddToViewport` _returnvalue 0)))

(event `self.TriggerBox.OnComponentEndOverlap`
  (params (OverlappedComponent :type "PrimitiveComponent Object Reference") (OtherActor :type "Actor Object Reference") (OtherComp :type "PrimitiveComponent Object Reference") (OtherBodyIndex :type Integer))
  (if (== (`GameplayStatics.GetPlayerCharacter` 0) OtherActor)
    (`/Engine/EditorBlueprintResources/StandardMacros.IsValid` (stale `self.TriggerBox.OnComponentBeginOverlap` _returnvalue)
      (:`Is Valid`
        (`Widget.RemoveFromParent` (stale `self.TriggerBox.OnComponentBeginOverlap` _returnvalue))))))

(fn `UserConstructionScript`
  (`parent.UserConstructionScript`))