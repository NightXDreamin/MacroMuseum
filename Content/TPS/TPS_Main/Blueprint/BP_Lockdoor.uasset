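; BP_Lockdoor is a door actor that slides its Door component toward a target relative location.
; Every Tick, MoveDoor eases the component toward TargetLocation with a frame-time-scaled VInterpTo, without sweeping.
; StartMove sets TargetLocation to the relative origin, which the door then glides to; nothing in this graph calls it.
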(event `self.ReceiveTick`
  (params (DeltaSeconds :type "Float (single-precision)"))
  (`self.MoveDoor`))

(fn `MoveDoor`
  (`SceneComponent.K2_SetRelativeLocation` (`self.Door`) (`KismetMathLibrary.VInterpTo` (`SceneComponent.RelativeLocation` (`self.Door`)) (`self.TargetLocation`) (`GameplayStatics.GetWorldDeltaSeconds`) 3.0) false false))

(fn `StartMove`
  (set `self.TargetLocation` (0.0 0.0 0.0)))

(fn `UserConstructionScript`)