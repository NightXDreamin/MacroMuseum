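; BP_PickupBase is a pickup base Blueprint that shows an on-screen widget while the player is within its collision volume.
; Begin overlap with player character 0 creates a widget from the Class value and adds it to the viewport.
; End overlap removes that widget if it is still valid.
; The graphs contain no item collection logic, and the construction script is empty.
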(event `self.Collision.OnComponentBeginOverlap`
  (params (OverlappedComponent :type "PrimitiveComponent Object Reference") (OtherActor :type "Actor Object Reference") (OtherComp :type "PrimitiveComponent Object Reference") (OtherBodyIndex :type Integer) (bFromSweep :type Boolean) (SweepResult :type "HitResult Structure (by ref)"))
  (if (== OtherActor (`GameplayStatics.GetPlayerCharacter` 0))
    (bind _returnvalue (`|CreateWidget` (`self.Class`)))
    (`UserWidget.AddToViewport` _returnvalue 0)))

(event `self.Collision.OnComponentEndOverlap`
  (params (OverlappedComponent :type "PrimitiveComponent Object Reference") (OtherActor :type "Actor Object Reference") (OtherComp :type "PrimitiveComponent Object Reference") (OtherBodyIndex :type Integer))
  (if (== (`GameplayStatics.GetPlayerCharacter` 0) OtherActor)
    (`/Engine/EditorBlueprintResources/StandardMacros.IsValid` (stale `self.Collision.OnComponentBeginOverlap` _returnvalue)
      (:`Is Valid`
        (`Widget.RemoveFromParent` (stale `self.Collision.OnComponentBeginOverlap` _returnvalue))))))

(fn `UserConstructionScript`)