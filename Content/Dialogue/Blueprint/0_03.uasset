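; Dialogue actor that shows a character name text and opens a conversation once when the player character enters its trigger.
; The trigger overlap and StartConversation event share one DoOnce, which calls OpenConversation on the ConversationComponent.
; On close, it hides the mouse cursor, restores game-only input and calls CallConversationIsEnd.
; The construction script fills the name text from CharacterName, and SetInteractableState toggles its visibility.
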(event `self.SetInteractableState`
  (params (b_CanShowInteract :type Boolean))
  (bind _txt_charactername (`self.Txt_CharacterName`))
  (if b_CanShowInteract
    (`SceneComponent.SetVisibility` _txt_charactername true false)
    (else
      (`SceneComponent.SetVisibility` _txt_charactername false false))))

(event `Start Conversation`
  (`/Engine/EditorBlueprintResources/StandardMacros.DoOnce` false :!label _label
    (:`Completed`
      (`/Game/Dialogue/Blueprint/AC_Dialogue_Base.OpenConversation` (`self.ConversationComponent`)))))

(event `self.trigger.OnComponentBeginOverlap`
  (params (OverlappedComponent :type "PrimitiveComponent Object Reference") (OtherActor :type "Actor Object Reference") (OtherComp :type "PrimitiveComponent Object Reference") (OtherBodyIndex :type Integer) (bFromSweep :type Boolean) (SweepResult :type "HitResult Structure (by ref)"))
  (if (== OtherActor (`GameplayStatics.GetPlayerCharacter` 0))
    (goto _label)))

(event `self.ConversationClosed`
  (`self.ConversationEnd`)
  (`self.ConversationIsEnd`))

(fn `ConversationEnd`
  (bind _returnvalue (`GameplayStatics.GetPlayerController` 0))
  (set `PlayerController.bShowMouseCursor` false _returnvalue)
  (`WidgetBlueprintLibrary.SetInputMode_GameOnly` _returnvalue))

(fn `UserConstructionScript`
  (`TextRenderComponent.K2_SetText` (`self.Txt_CharacterName`) (`self.Character_Name`)))