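; AC_Dialogue_Quiny scripts the NPC Quiny's branching conversation by overriding the parent Dialogue function.
; DialogueTreeIndex picks the opening branch; AddDialogue nodes chain on Pass Through through the chosen option, while one Updated output switches Ultra Dynamic Weather to a blizzard.
; Endings clear or rewind progress before closing, and one moves later talks to a branch with randomized lines.
; Chinese comments and unwired example nodes document the authoring pattern.
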(fn `Dialogue`
  (`parent.Dialogue`)
  (switch `int` (`self.DialogueTreeIndex`) ; 初始分支，默认为0
    (:`0`
      (bind (_state _optionindex) (`self.AddDialogue` "Quiny" "Hi, Good morning" (`|MakeArray` "Hi" "Good morning" :!type "Text"))) ; 分支0—阶段1
      (switch `/Game/Dialogue/Enum_DialogueState` _state ; 当选择完成后会触发PassThrough，选项出现时则触发Updated
        (:`NewEnumerator0`
          (switch `int` _optionindex
            (:`0`
              (bind (_state_2 _optionindex_2) (`self.AddDialogue` "Quiny" "Hello" (`|MakeArray` "See you later!" "Do you know about zzz?" :!type "Text"))) ; 分支0-阶段2
              (switch `/Game/Dialogue/Enum_DialogueState` _state_2
                (:`NewEnumerator0`
                  (switch `int` _optionindex_2
                    (:`0`
                      (`self.ClearDialogueProgress`) ; 清除当前进度，从头开始判定
                      (`self.SetDialogueTreeIndex` 1) ; 若清除进度后再次对话，将初始分支处的选择强制为所输数字
                      (`self.CloseConversation`))
                    (:`1`
                      (`self.RemoveDialogueProgress` 0) ; 本分支无清除，此节点作用为回跳所输数字次的阶段，举例：本阶段为分支0阶段2，因此若填写0
                      (`self.CloseConversation`) ; 下次互动则仍跳入分支0阶段2，若填写1，下次分支则跳入分支0阶段1
                    )))))
            (:`1`
              (bind (_state_3 _optionindex_3) (`self.AddDialogue` "Quiny" "Have a nice day, buddy" (`|MakeArray` "You too!" "Hooray!!" :!type "Text")))
              (switch `/Game/Dialogue/Enum_DialogueState` _state_3
                (:`NewEnumerator0`
                  (switch `int` _optionindex_3))
                (:`NewEnumerator1`
                  (bind _returnvalue (`GameplayStatics.GetActorOfClass` "/Game/UltraDynamicSky/Blueprints/Ultra_Dynamic_Weather.Ultra_Dynamic_Weather_C"))
                  (set `/Game/UltraDynamicSky/Blueprints/Ultra_Dynamic_Weather.Weather` "/Game/UltraDynamicSky/Blueprints/Weather_Effects/Weather_Presets/Snow_Blizzard.Snow_Blizzard" _returnvalue))))))))
    (:`1`
      (bind (_state_4 _optionindex_4) (`self.AddDialogue` "Quiny" (select `int` (`KismetMathLibrary.RandomIntegerInRange` 0 1) :`0` "You are not allowed to be here" :`1` "Who are you!" :!type "Text") (`|MakeArray` "Continue" :!type "Text")))
      (switch `/Game/Dialogue/Enum_DialogueState` _state_4
        (:`NewEnumerator0`
          (switch `int` _optionindex_4
            (:`0`
              (`self.ClearDialogueProgress`)
              (`self.CloseConversation`))))))))