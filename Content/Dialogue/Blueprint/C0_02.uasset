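; Dialogue Blueprint C0_02: a short protagonist monologue noting that the door is blocked and the gun is missing, likely dropped on top of the statue.
; The Dialogue override calls its parent, then switches on DialogueTreeIndex, where only branch 0 is defined.
; That branch chains three single-option AddDialogue nodes through their Pass Through state, then calls CloseConversation.
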(fn `Dialogue`
  (`parent.Dialogue`)
  (switch `int` (`self.DialogueTreeIndex`) ; 初始分支，默认为0
    (:`0`
      (bind (_state _optionindex) (`self.AddDialogue` "我" "门被挡住了" (`|MakeArray` "..." :!type "Text")))
      (switch `/Game/Dialogue/Enum_DialogueState` _state
        (:`NewEnumerator0`
          (switch `int` _optionindex
            (:`0`
              (bind (_state_2 _optionindex_2) (`self.AddDialogue` "我" "我的枪也不见了。" (`|MakeArray` "..." :!type "Text")))
              (switch `/Game/Dialogue/Enum_DialogueState` _state_2
                (:`NewEnumerator0`
                  (switch `int` _optionindex_2
                    (:`0`
                      (bind (_state_3 _optionindex_3) (`self.AddDialogue` "我" "好像掉在了那个雕像顶上。" (`|MakeArray` "....." :!type "Text")))
                      (switch `/Game/Dialogue/Enum_DialogueState` _state_3
                        (:`NewEnumerator0`
                          (switch `int` _optionindex_3
                            (:`0`
                              (`self.CloseConversation`))))))))))))))))