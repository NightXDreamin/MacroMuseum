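; Base NPC Blueprint for the dialogue system, with a name label that signals when the character can be interacted with.
; The construction script writes CharacterName into the TxtCharacterName component.
; SetInteractableState shows or hides that label, and ConversationClosed notifies the stored InteractInstigator through ConversationClosedMessage.
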(event `/Game/Dialogue/UI/BI_Interactable.SetInteractableState`
  (params (b_CanShowInteract :type Boolean))
  (bind _txt_charactername (`self.Txt_CharacterName`))
  (if b_CanShowInteract
    (`SceneComponent.SetVisibility` _txt_charactername true false)
    (else
      (`SceneComponent.SetVisibility` _txt_charactername false false))))

(event `/Game/Dialogue/UI/BI_Interactable.ConversationClosed`
  (message `/Game/Dialogue/UI/BI_Interactable.ConversationClosed` (`self.Interact_Instigator`)))

(fn `UserConstructionScript`
  (`TextRenderComponent.K2_SetText` (`self.Txt_CharacterName`) (`self.Character_Name`)))