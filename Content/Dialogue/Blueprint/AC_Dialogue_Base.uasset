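; Base dialogue component that runs branching conversations, with the tree defined by child classes overriding Dialogue.
; Opening creates the lower-half dialogue widget in UI-only input; closing removes it and notifies the owner.
; Each progression replays the tree from the start: AddDialogue returns saved choices by running index or displays the first unanswered line.
; Helpers clear or rewind progress, switch tree index, and play montages on the owner's skeletal mesh.
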(event `PlayAnimation`
  (params (MontageToPlay :type "AnimMontage Object Reference"))
  (`|PlayMontage` (`Actor.GetComponentByClass` (`self.GetOwner`) "/Script/Engine.SkeletalMeshComponent") MontageToPlay))

(fn `AddDialogue`
  (params (Speaker :type Text) (Dialogue :type Text) (Option :type "Array of Text"))
  (returns (State :type "/Game/Dialogue/Enum_DialogueState Enum") (OptionIndex :type Integer))
  (bind _result (`/Engine/EditorBlueprintResources/StandardMacros.IncrementInt` (`self.DialogueIndex`))
    (:`  `
      (bind (_value _returnvalue) (`BlueprintMapLibrary.Map_Find` (`self.DialogueProgress`) _result))
      (if _returnvalue
        (return "NewEnumerator0" _value)
        (else
          (`/Game/Dialogue/UI/WB_Dialogue_LowerHalf.UpdateDialogueText` (`self.DialogueWidget`) (`self.DialogueIndex`) (`local.Speaker`) (`local.Dialogue`) (`local.Option`))
          (return "NewEnumerator1" 0))))))

(fn `ClearDialogueProgress`
  (`BlueprintMapLibrary.Map_Clear` (`self.DialogueProgress`)))

(fn `CloseConversation`
  (`Widget.RemoveFromParent` (`self.DialogueWidget`))
  (message `/Game/Dialogue/UI/BI_Interactable.ConversationClosed` (`self.GetOwner`)))

(fn `Dialogue`)

(fn `OpenConversation`
  (bind _returnvalue (`GameplayStatics.GetPlayerController` 0))
  (bind _returnvalue_2 (`|CreateWidget` "/Game/Dialogue/UI/WB_Dialogue_LowerHalf.WB_Dialogue_LowerHalf_C" null self))
  (bind _output_get (set `self.DialogueWidget` _returnvalue_2))
  (`UserWidget.AddToViewport` _output_get 0)
  (`self.ProgressDialogue`)
  (set `PlayerController.bShowMouseCursor` true _returnvalue)
  (`WidgetBlueprintLibrary.SetInputMode_UIOnlyEx` _returnvalue null))

(fn `ProgressDialogue`
  (set `self.DialogueIndex` -1)
  (`self.Dialogue`))

(fn `RemoveDialogueProgress`
  (params (ProgressSteps :type Integer))
  (for _index (range (+ ProgressSteps 1))
    (`BlueprintMapLibrary.Map_Remove` (`self.DialogueProgress`) (- (`self.DialogueIndex`) _index))))

(fn `SetDialogueTreeIndex`
  (params (DialogueTreeIndex :type Integer))
  (set `self.DialogueTreeIndex` DialogueTreeIndex)
  (`self.ClearDialogueProgress`))

(fn `UpdateSelectedOption`
  (params (ProgressIndex :type "Integer (by ref)") (OptionIndex :type "Integer (by ref)"))
  (`BlueprintMapLibrary.Map_Add` (`self.DialogueProgress`) ProgressIndex OptionIndex)
  (`self.ProgressDialogue`))