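; BP_Support is a resizable support prop that, when shrunk, lets an optional linked FallDecor piece fall by enabling its physics.
; SetSize handles only the shrink mode, suspending its own mesh physics and starting a looping timer.
; The first timer tick runs TickSize, then clears the timer, signals ShrinkDone and restores physics.
; Outline highlighting switches itself off through a short retriggerable delay unless refreshed.
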(event `self.ReceiveBeginPlay`
  (`parent.ReceiveBeginPlay`))

(event `self.SetSize`
  (params (SizeMode :type "/Game/Resize/Enumeration/ESizeMode Enum" :default "NewEnumerator0"))
  (if (== SizeMode 1)
    (bind _falldecor (`self.FallDecor`)
      (:`then`
        (`PrimitiveComponent.SetSimulatePhysics` (`/Game/TPS/TPS_Main/Blueprint/BP_FallDecor.Cube` _falldecor) true))
      (:`else`
        _))
    (`PrimitiveComponent.SetSimulatePhysics` (`self.StaticMesh`) false)
    (`self.ChangeSize` SizeMode)
    (bind _returnvalue (`KismetSystemLibrary.K2_SetTimerDelegate` (delegate `CustomEvent`) 0.1 true))))

(event `CustomEvent`
  (`self.TickSize`)
  (if true
    (`KismetSystemLibrary.K2_ClearAndInvalidateTimerHandle` (stale `self.SetSize` _returnvalue))
    (`self.ShrinkDone`)
    (`PrimitiveComponent.SetSimulatePhysics` (`self.StaticMesh`) true)))

(event `self.EnableOutline`
  (params (`Enable?` :type Boolean))
  (`self.EnableOutlineMesh` `Enable?`)
  (`KismetSystemLibrary.RetriggerableDelay` 0.1)
  (`self.EnableOutlineMesh` false))

(fn `UserConstructionScript`
  (`parent.UserConstructionScript`))