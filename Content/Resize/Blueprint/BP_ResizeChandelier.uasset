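; Resizable chandelier actor that falls under physics and kills any ALS_Enemy that overlaps its box.
; SetSize either changes its size or, when resizing is off, enables physics immediately.
; After a resize, a looping timer polls until the target scale is reached, then enables physics and destroys the actor five seconds later.
; Outline highlighting switches itself off through a short retriggerable delay unless refreshed.
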(event `self.Box.OnComponentBeginOverlap`
  (params (OverlappedComponent :type "PrimitiveComponent Object Reference") (OtherActor :type "Actor Object Reference") (OtherComp :type "PrimitiveComponent Object Reference") (OtherBodyIndex :type Integer) (bFromSweep :type Boolean) (SweepResult :type "HitResult Structure (by ref)"))
  (if (== (`GameplayStatics.GetObjectClass` OtherActor) "/Game/TPS/TPS_Main/AI/ALS_Enemy.ALS_Enemy_C")
    (bind _asals_enemy (cast `/Game/TPS/TPS_Main/AI/ALS_Enemy` OtherActor))
    (`/Game/TPS/TPS_Main/AI/ALS_Enemy.GetKilled` _asals_enemy)))

(event `/Game/Resize/Blueprint/BPI_Resize.EnableOutline`
  (params (`Enable?` :type Boolean))
  (`self.EnableOutlineMesh` `Enable?`)
  (`KismetSystemLibrary.RetriggerableDelay` 0.1)
  (`self.EnableOutlineMesh` false))

(event `/Game/Resize/Blueprint/BPI_Resize.SetSize`
  (params (SizeMode :type "/Game/Resize/Enumeration/ESizeMode Enum" :default "NewEnumerator0"))
  (if (`self.bIfResize`)
    (`self.ChangeSize` SizeMode)
    (bind _returnvalue (`KismetSystemLibrary.K2_SetTimerDelegate` (delegate `CustomEvent`) 0.1 true))
    (else
      (`PrimitiveComponent.SetSimulatePhysics` (`self.StaticMesh`) true))))

(event `CustomEvent`
  (if (== (`self.GetActorScale3D`) (* (`self.TargetScale`) (`self.UserScale`)))
    (`KismetSystemLibrary.K2_ClearAndInvalidateTimerHandle` (stale `/Game/Resize/Blueprint/BPI_Resize.SetSize` _returnvalue))
    (`PrimitiveComponent.SetSimulatePhysics` (`self.StaticMesh`) true)
    (`KismetSystemLibrary.Delay` 5.0)
    (`self.K2_DestroyActor`)))

(fn `UserConstructionScript`
  (`parent.UserConstructionScript`))