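; BP_TempResizeBase is a base actor that can be temporarily enlarged or shrunk and highlighted with an outline.
; SetSize steps a clamped Small/Middle/Large state, then restores Middle after a three-second delay.
; Tick smoothly interpolates the actor's scale toward that state's multiple of its construction-time scale.
; An outline copy of the static mesh uses M_Outline, and EnableOutline auto-hides it unless continually re-triggered.
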(event `self.ReceiveTick`
  (params (DeltaSeconds :type "Float (single-precision)"))
  (`self.TickSize`))

(event `self.SetSize`
  (params (SizeMode :type "/Game/Resize/Enumeration/ESizeMode Enum" :default "NewEnumerator0"))
  (`self.ChangeSize` SizeMode)
  (`KismetSystemLibrary.Delay` 3.0)
  (set `self.Size` "NewEnumerator1")
  (`self.SetActorSize`))

(event `self.EnableOutline`
  (params (`Enable?` :type Boolean))
  (`self.EnableOutlineMesh` `Enable?`)
  (`KismetSystemLibrary.RetriggerableDelay` 0.1)
  (`self.EnableOutlineMesh` false))

(fn `ChangeSize`
  (params (Selection :type "/Game/Resize/Enumeration/ESizeMode Enum" :default "NewEnumerator0"))
  (switch `/Game/Resize/Enumeration/ESizeMode` Selection
    (:`NewEnumerator0`
      (set `self.Size` (cast `/Game/Resize/Enumeration/ESize` (`KismetMathLibrary.Conv_IntToByte` (`KismetMathLibrary.Clamp` (+ (`KismetMathLibrary.Conv_ByteToInt` (`self.Size`)) 1) 0 2)))))
    (:`NewEnumerator1`
      (set `self.Size` (cast `/Game/Resize/Enumeration/ESize` (`KismetMathLibrary.Conv_IntToByte` (`KismetMathLibrary.Clamp` (- (`KismetMathLibrary.Conv_ByteToInt` (`self.Size`)) 1) 0 2))))))
  (`self.SetActorSize`))

(fn `EnableOutlineMesh`
  (params (`Enable?` :type Boolean))
  (bind _outline (`self.Outline`))
  (`/Engine/EditorBlueprintResources/StandardMacros.IsValid` _outline
    (:`Is Valid`
      (`SceneComponent.SetVisibility` _outline `Enable?` false))))

(fn `SetActorSize`
  (set `self.TargetScale` (* (`self.UserScale`) (select `/Game/Resize/Enumeration/ESize` (`self.Size`) :`NewEnumerator0` (0.33 0.33 0.33) :`NewEnumerator1` (1.0 1.0 1.0) :`NewEnumerator2` (3.0 3.0 3.0) :!type "Vector Structure"))))

(fn `TickSize`
  (`self.SetActorScale3D` (`KismetMathLibrary.VInterpTo` (`self.GetActorScale3D`) (`self.TargetScale`) (`GameplayStatics.GetWorldDeltaSeconds`) 10.0)))

(fn `UserConstructionScript`
  (bind _outline (`self.Outline`))
  (bind _staticmesh (`StaticMeshComponent.StaticMesh` (`self.StaticMesh`)))
  (`/Engine/EditorBlueprintResources/StandardMacros.IsValid` _staticmesh
    (:`Is Valid`
      (`StaticMeshComponent.SetStaticMesh` _outline _staticmesh)
      (`PrimitiveComponent.SetMaterial` _outline 0 "/Game/Resize/Material/M_Outline.M_Outline")
      (bind _output_get (set `self.UserScale` (`self.GetActorScale3D`)))
      (set `self.TargetScale` _output_get))))