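; BP_TempBox is a resizable box whose size changes are temporary.
; SetSize applies the requested mode through ChangeSize, then after a three-second delay resets Size to a fixed enum value and calls SetActorSize.
; EnableOutline sets the outline mesh state and uses a retriggerable delay to switch it off shortly after the last call, so a highlight persists only while calls keep arriving.
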(event `/Game/Resize/Blueprint/BPI_Resize.SetSize`
  (params (SizeMode :type "/Game/Resize/Enumeration/ESizeMode Enum" :default "NewEnumerator0"))
  (`self.ChangeSize` SizeMode)
  (`KismetSystemLibrary.Delay` 3.0)
  (set `self.Size` "NewEnumerator1")
  (`self.SetActorSize`))

(event `/Game/Resize/Blueprint/BPI_Resize.EnableOutline`
  (params (`Enable?` :type Boolean))
  (`self.EnableOutlineMesh` `Enable?`)
  (`KismetSystemLibrary.RetriggerableDelay` 0.1)
  (`self.EnableOutlineMesh` false))

(fn `UserConstructionScript`
  (`parent.UserConstructionScript`))