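; BP_SequenceManager is a trigger actor that stages a scripted story beat combining a door, a level sequence and an NPC conversation.
; When the player leaves its Box, a DoOnce starts LockDoor moving, plays LS_0_03 through Sequence and binds Conversation to its finish.
; The Conversation event starts the NPC's dialogue and re-enables player input.
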(event `self.Box.OnComponentEndOverlap`
  (params (OverlappedComponent :type "PrimitiveComponent Object Reference") (OtherActor :type "Actor Object Reference") (OtherComp :type "PrimitiveComponent Object Reference") (OtherBodyIndex :type Integer))
  (bind _sequence (`self.Sequence`))
  (if (== OtherActor (`GameplayStatics.GetPlayerCharacter` 0))
    (`/Engine/EditorBlueprintResources/StandardMacros.DoOnce` false
      (:`Completed`
        (`/Game/TPS/TPS_Main/Blueprint/BP_Lockdoor.StartMove` (`self.LockDoor`))
        (`/Game/Sequence/Blueprint/BP_TriggerBox.StartSequence` _sequence "/Game/Sequence/LS_0_03.LS_0_03")
        (add `/Game/Sequence/Blueprint/BP_TriggerBox.Finished` _sequence (delegate `Conversation`))))))

(event `CustomEvent`
  (params (OverlappedComponent :type "PrimitiveComponent Object Reference") (OtherActor :type "Actor Object Reference") (OtherComp :type "PrimitiveComponent Object Reference") (OtherBodyIndex :type Integer) (bFromSweep :type Boolean) (SweepResult :type "HitResult Structure (by ref)")))

(event `self.Box.OnComponentBeginOverlap`
  (params (OverlappedComponent :type "PrimitiveComponent Object Reference") (OtherActor :type "Actor Object Reference") (OtherComp :type "PrimitiveComponent Object Reference") (OtherBodyIndex :type Integer) (bFromSweep :type Boolean) (SweepResult :type "HitResult Structure (by ref)")))

(event `Conversation`
  (`/Game/Dialogue/Blueprint/0_04.Start Conversation` (`self.ConversationNpc`))
  (`self.EnableInput` (`GameplayStatics.GetPlayerCharacter` 0) (`GameplayStatics.GetPlayerController` 0)))

(fn `UserConstructionScript`)