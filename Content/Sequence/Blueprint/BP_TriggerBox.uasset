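; Trigger box actor that plays a Level Sequence once and signals when it ends.
; StartSequence stores the given sequence and continues into a DoOnce, which the player character overlapping the box also enters.
; The first arrival creates a sequence player, plays it and binds its OnFinished to End, which calls the Finished dispatcher.
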(event `StartSequence`
  (params (LevelSequence :type "LevelSequence Object Reference"))
  (set `self.Level Sequence` LevelSequence)
  (`/Engine/EditorBlueprintResources/StandardMacros.DoOnce` false :!label _label
    (:`Completed`
      (bind (_outactor _returnvalue) (`LevelSequencePlayer.CreateLevelSequencePlayer` (`self.Level Sequence`)))
      (`MovieSceneSequencePlayer.Play` _returnvalue)
      (add `MovieSceneSequencePlayer.OnFinished` _returnvalue (delegate `End`)))))

(event `self.Box.OnComponentBeginOverlap`
  (params (OverlappedComponent :type "PrimitiveComponent Object Reference") (OtherActor :type "Actor Object Reference") (OtherComp :type "PrimitiveComponent Object Reference") (OtherBodyIndex :type Integer) (bFromSweep :type Boolean) (SweepResult :type "HitResult Structure (by ref)"))
  (if (== OtherActor (`GameplayStatics.GetPlayerCharacter` 0))
    (goto _label)))

(event `End`
  (`self.Finished`))

(fn `UserConstructionScript`)